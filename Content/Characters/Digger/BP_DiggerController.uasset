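; BP_DiggerController is the player controller that turns input into actions on the possessed Digger character.
; On possess, it casts the pawn to BP_Digger, stores the reference, and adds IMC_Default to the Enhanced Input subsystem.
; Move and Look input actions pass their values to the Digger's own functions, and Fire calls DiggerFire when the action completes.
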(event `self.ReceivePossess`
  (params (PossessedPawn :type "Pawn Object Reference"))
  ;[1 1 1] This is important! Add Mapping context is what actually makes the EnhancedInputSystem work lol
  (bind _asbp_digger (cast `/Game/Characters/Digger/BP_Digger` PossessedPawn))
  (set `self.As BP Digger` _asbp_digger)
  (`EnhancedInputSubsystemInterface.AddMappingContext` (pcsubsystem `EnhancedInputLocalPlayerSubsystem` (`GameplayStatics.GetPlayerController` 0)) "/Game/Input/IMC_Default.IMC_Default" 0 (struct)))

(event `EnhancedInput|/Game/Input/Actions/IA_Move`
  (params (ActionValue :type "Vector2D Structure") (ElapsedSeconds :type "Float (double-precision)") (TriggeredSeconds :type "Float (double-precision)") (InputAction :type "InputAction Object Reference" :default "/Game/Input/Actions/IA_Move.IA_Move"))
  (:`Triggered`
    (`/Game/Characters/Digger/BP_Digger.Digger_Move` (`self.As BP Digger`) ActionValue)))

(event `EnhancedInput|/Game/Input/Actions/IA_Look`
  (params (ActionValue :type "Vector2D Structure") (ElapsedSeconds :type "Float (double-precision)") (TriggeredSeconds :type "Float (double-precision)") (InputAction :type "InputAction Object Reference" :default "/Game/Input/Actions/IA_Look.IA_Look"))
  (:`Triggered`
    (`/Game/Characters/Digger/BP_Digger.Digger_Look` (`self.As BP Digger`) ActionValue)))

(event `EnhancedInput|/Game/Input/Actions/IA_Fire`
  (params (ActionValue :type Boolean) (ElapsedSeconds :type "Float (double-precision)") (TriggeredSeconds :type "Float (double-precision)") (InputAction :type "InputAction Object Reference" :default "/Game/Input/Actions/IA_Fire.IA_Fire"))
  (:`Completed`
    (`/Game/Characters/Digger/BP_Digger.Digger_Fire` (`self.As BP Digger`))))

(fn `UserConstructionScript`)