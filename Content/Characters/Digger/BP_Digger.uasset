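; Digger character Blueprint with camera-relative movement, independent aiming and projectile firing.
; Move and Look convert 2D input to world space through a shared helper fed by camera forward and right vectors.
; Move applies the normalized direction as movement input, while Look yaws only the mesh to the vector's heading.
; Fire spawns a BP_DiggerProjectile at the ProjectileArrow transform, regardless of collisions.
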(fn `Digger_Fire`
  (`|SpawnActorFromClass` "/Game/Characters/Digger/BP_DiggerProjectile.BP_DiggerProjectile_C" (`SceneComponent.K2_GetComponentToWorld` (`self.ProjectileArrow`)) "AlwaysSpawn" "MultiplyWithRoot" null null))

(fn `Digger_Look`
  (params (`Input Vector` :type "Vector2D Structure"))
  (bind (_forward_vector _right_vector) (`self.Get Camera Basis Vectors`))
  (bind _returnvalue (`self.Input Vector to World Vector` `Input Vector` _forward_vector _right_vector))
  (`SceneComponent.K2_SetRelativeRotation` (`self.Mesh`) (`KismetMathLibrary.RotatorFromAxisAndAngle` (0.0 0.0 -1.0) (+ (`KismetMathLibrary.RadiansToDegrees` (`KismetMathLibrary.Vector_HeadingAngle` _returnvalue)) 90.0)) false false))

(fn `Digger_Move`
  (params (`Input Vector` :type "Vector2D Structure"))
  (bind (_forward_vector _right_vector) (`self.Get Camera Basis Vectors`))
  (bind _returnvalue (`self.Input Vector to World Vector` `Input Vector` _forward_vector _right_vector))
  (`self.AddMovementInput` (`KismetMathLibrary.Normal` _returnvalue)))

(fn `Input Vector to World Vector`
  (params (InputVector :type "Vector2D Structure") (CameraForward :type "Vector Structure") (CameraRight :type "Vector Structure"))
  (returns (ReturnValue :type "Vector Structure"))
  (bind (_x _y) (`KismetMathLibrary.BreakVector2D` InputVector))
  (return (+ (* _y CameraForward) (* _x CameraRight))))

(fn `UserConstructionScript`)